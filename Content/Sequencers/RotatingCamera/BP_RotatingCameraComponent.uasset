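; Actor component for a Level Sequence Actor that runs a looping camera sequence while a Picross puzzle is in its solved state.
; On BeginPlay it finds the BP_Picross actor and binds to its Solved and PuzzleLoaded events, unbinding them on EndPlay.
; Solved loops the owner's sequence player indefinitely, and PuzzleLoaded sends it to the end and stops it.
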(event Custom|Event%20Puzzle%20Loaded
  ;[1 1 1] Bind Loaded puzzle to stop camera loop
  (bind _aslevel_sequence_actor (Utilities|Casting|CastToLevelSequenceActor (Components|GetOwner)))
  (Class|MovieSceneSequencePlayer|GotoEndandStop (Variables|/Script/LevelSequence.LevelSequenceActor|GetSequencePlayer _aslevel_sequence_actor)))

(event Custom|Event%20Solved
  ;[1 1 1] Bind Solved puzzle to play camera loop
  (bind _aslevel_sequence_actor (Utilities|Casting|CastToLevelSequenceActor (Components|GetOwner)))
  (Class|MovieSceneSequencePlayer|PlayLooping (Variables|/Script/LevelSequence.LevelSequenceActor|GetSequencePlayer _aslevel_sequence_actor) -1))

(event EventBeginPlay
  (bind _returnvalue (Actor|GetActorOfClass "/Game/Behaviour/BP_Picross.BP_Picross_C"))
  ;[1 1 1] Bind Solved puzzle to play camera loop
  (EventDispatchers|BindEventtoSolvedEvent _returnvalue (delegate Custom|Event%20Solved))
  ;[1 1 1] Bind Loaded puzzle to stop camera loop
  (EventDispatchers|BindEventtoPuzzleLoaded _returnvalue (delegate Custom|Event%20Puzzle%20Loaded)))

(event EventEndPlay
  (params (EndPlayReason :type EEndPlayReason%20Enum :default "Destroyed"))
  (bind _returnvalue (Actor|GetActorOfClass "/Game/Behaviour/BP_Picross.BP_Picross_C"))
  (EventDispatchers|UnbindEventfromSolvedEvent _returnvalue (delegate Custom|Event%20Solved))
  (EventDispatchers|UnbindEventfromPuzzleLoaded _returnvalue (delegate Custom|Event%20Puzzle%20Loaded)))